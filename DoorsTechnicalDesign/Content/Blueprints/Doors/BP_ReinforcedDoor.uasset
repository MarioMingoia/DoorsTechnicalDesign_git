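; Reinforced door Blueprint that is locked and unlocked through a linked lever instead of direct interaction, as its Interact function returns false.
; SetLock runs on construction and BeginPlay, checking the door type data asset to set the alternative-unlock flag and show or hide the point light and lever.
; Unlock and lock events recolour the light green or red, set the lock flag and open or close the door.
; Leaving the collision zone tells the lever to handle locking.
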(event OnComponentEndOverlap(BC_DoorCollision)
  (params (OverlappedComponent :type Primitive%20Component%20Object%20Reference) (OtherActor :type Actor%20Object%20Reference) (OtherComp :type Primitive%20Component%20Object%20Reference) (OtherBodyIndex :type Integer))
  ;[1 1 1] when leaving the trigger zone, cast to lever and lock it
  ;;[1 0.6445 0] MM - Try and avoid using casting
  (bind _asbp_lever (Utilities|Casting|CastToBP_Lever (Variables|Default|Getact_Lever)))
  (Default|HandleLock _asbp_lever))

(event Custom|UnlockDoor
  ;[1 1 1] Calls custom events
  ;[1 1 1] Change colour of light
  (Rendering|Components|Light|SetLightColor (Variables|Default|GetPointLight) "(R=0.086861,G=1.000000,B=0.000000,A=1.000000)" true)
  ;[1 1 1] change the lock boolean
  (Variables|Default|Setbol_Lock false)
  ;[1 1 1] calls open/ close event
  (CallFunction|OpenDoor))

(event Custom|LockDoor
  ;[1 1 1] Calls custom events
  ;[1 1 1] Change colour of light
  (Rendering|Components|Light|SetLightColor (Variables|Default|GetPointLight) "(R=1.000000,G=0.000000,B=0.000000,A=1.000000)" true)
  ;[1 1 1] change the lock boolean
  (Variables|Default|Setbol_Lock true)
  ;[1 1 1] calls open/ close event
  (CallFunction|CloseDoor))

(event EventBeginPlay
  (|CallParentFunction)
  (CallFunction|SetLock))

(fn ConstructionScript
  (|CallParentFunction)
  (CallFunction|SetLock))

(fn Interact
  (params (Interactor :type Character%20Object%20Reference))
  (return false))

(fn SetLock
  (bind _pointlight (Variables|Default|GetPointLight))
  (bind _act_lever (Variables|Default|Getact_Lever))
  (if (== (Variables|Default|GetBPDA_DoorType) "/Game/DataAssets/BPDA_ReinforcedDoor.BPDA_ReinforcedDoor")
    (bind _output_get (Variables|Default|Setbol_AlternativeUnlock true))
    (Development|PrintString (Utilities|String|ToString(Boolean) _output_get))
    (Rendering|SetVisibility _pointlight true false)
    (Rendering|SetActorHiddenInGame _act_lever false)
    (else
      (bind _output_get_2 (Variables|Default|Setbol_AlternativeUnlock false))
      (Development|PrintString (Utilities|String|ToString(Boolean) _output_get_2))
      (Rendering|SetVisibility _pointlight false false)
      (Rendering|SetActorHiddenInGame _act_lever true))))