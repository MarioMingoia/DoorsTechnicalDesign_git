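; Parent door Blueprint that players open, close, lock and unlock through Interact and Unlocking functions.
; A door-type data asset supplies mesh, material, sounds and optional gameplay settings at BeginPlay.
; A timeline lerps door yaw, choosing swing direction by player-to-door dot product when swing-away is set, and reacts to hit-box overlaps mid-motion.
; The interact trigger toggles prompts and auto-closes on exit, while timeline completion flips open state and can auto-lock.
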(event OnComponentBeginOverlap(BC_InteractCollision)
  (params (OverlappedComponent :type Primitive%20Component%20Object%20Reference) (OtherActor :type Actor%20Object%20Reference) (OtherComp :type Primitive%20Component%20Object%20Reference) (OtherBodyIndex :type Integer) (bFromSweep :type Boolean) (SweepResult :type Hit%20Result%20Structure%20%28by%20ref%29))
  ;[1 1 1] Displays
  (Development|PrintString "Entered trigger zone")
  (if (Variables|Default|Gameplay|Getbol_Lock)
    (Development|PrintString "door looked")
    (Rendering|SetVisibility (Variables|Default|GetTR_UnlockPromptFront) true false)
    (else
      (Rendering|SetVisibility (Variables|Default|GetTR_OpenPromptFront) true false)
      (Rendering|SetVisibility (Variables|Default|GetTR_UnlockPromptFront) false false)))
  ;[1 1 1] Sets bool value whether the player is still in collision zone
  (Variables|Default|Setbol_InTriggerZone true))

(event OnComponentEndOverlap(BC_InteractCollision)
  (params (OverlappedComponent :type Primitive%20Component%20Object%20Reference) (OtherActor :type Actor%20Object%20Reference) (OtherComp :type Primitive%20Component%20Object%20Reference) (OtherBodyIndex :type Integer))
  ;[1 1 1] Checks if actor has left collision area
  ;[1 1 1] Sets bool value whether the player is still in collision zone
  (Variables|Default|Setbol_InTriggerZone false)
  ;[1 1 1] Sets visibility to hide the text of prompt when exiting collision area
  (CallFunction|HideTooltips)
  ;[1 1 1] Checks if door is currently open
  (if (Variables|Default|Getbol_IsOpen)
    ;[1 1 1] Checks if door auto closes
    (if (Variables|Default|Gameplay|Getbol_AutoClose)
      ;[1 1 1] Open/ Close door in timeline
      (bind _track_door (Timeline|TL_OpenDoor Reverse)
        (:Update
          ;[1 1 1] Call custom collision event
          (CallFunction|PlayerDoorCollisionEvent)
          (Transformation|SetRelativeRotation (Variables|Default|GetSM_Door) (Math|Rotator|MakeRotator 0.0 0.0 (Math|Float|Lerp (Variables|Default|Getfl_ClosePos) (Variables|Default|Getfl_OpenPos) _track_door)) false false))
        (:Finished
          ;[1 1 1] Calls finished timeline event that handles auto locking and closing the door
          (CallFunction|FinishedTimeline))))))

(event OnComponentBeginOverlap(BC_HitCollision)
  (params (OverlappedComponent :type Primitive%20Component%20Object%20Reference) (OtherActor :type Actor%20Object%20Reference) (OtherComp :type Primitive%20Component%20Object%20Reference) (OtherBodyIndex :type Integer) (bFromSweep :type Boolean) (SweepResult :type Hit%20Result%20Structure%20%28by%20ref%29))
  ;[1 1 1] Checks if player has entered/ exit collision area of BC_CheckPlayerCollision
  (Development|PrintString "In collision")
  ;[1 1 1] Sets bol depending on if the player is in the collision area
  (Variables|Default|Setbol_PlayerDoorCollided true))

(event OnComponentEndOverlap(BC_HitCollision)
  (params (OverlappedComponent :type Primitive%20Component%20Object%20Reference) (OtherActor :type Actor%20Object%20Reference) (OtherComp :type Primitive%20Component%20Object%20Reference) (OtherBodyIndex :type Integer))
  ;[1 1 1] Checks if player has entered/ exit collision area of BC_CheckPlayerCollision
  (Development|PrintString "Out collision")
  ;[1 1 1] Sets bol depending on if the player is in the collision area
  (Variables|Default|Setbol_PlayerDoorCollided false))

(event Custom|OpenDoor
  ;[1 1 1] Door events
  ;[1 1 1] Check and call the way the door swings
  (if (Variables|Default|Gameplay|Getbol_SwingAway)
    (CallFunction|Swinging))
  ;[1 1 1] Door unlocking
  (if (Variables|Default|Gameplay|Getbol_Lock)
    (Development|PrintString "Failed to unlock door")
    (else
      (Audio|PlaySoundatLocation (Variables|Default|Getsw_Unlock) (Transformation|GetActorForwardVector) "0, 0, 0" 1.0 1.0 0.0 0 0 0 0)
      ;[1 1 1] Sets visibility to hide the text of prompt when exiting collision area
      (CallFunction|HideTooltips)
      ;[1 1 1] Plays audio
      (Audio|PlaySoundatLocation (Variables|Default|Getsw_Open) (Transformation|GetActorForwardVector) "0, 0, 0" 1.0 1.0 0.0 0 0 0 0)
      ;[1 1 1] Open/ Close door in timeline
      (bind _track_door (Timeline|TL_OpenDoor Play)
        (:Update
          ;[1 1 1] Call custom collision event
          (CallFunction|PlayerDoorCollisionEvent)
          (Transformation|SetRelativeRotation (Variables|Default|GetSM_Door) (Math|Rotator|MakeRotator 0.0 0.0 (Math|Float|Lerp (Variables|Default|Getfl_ClosePos) (Variables|Default|Getfl_OpenPos) _track_door)) false false))
        (:Finished
          ;[1 1 1] Calls finished timeline event that handles auto locking and closing the door
          (CallFunction|FinishedTimeline))))))

(event Custom|CloseDoor
  ;[1 1 1] Door events
  ;[1 1 1] Sets visibility to hide the text of prompt when exiting collision area
  (CallFunction|HideTooltips)
  ;[1 1 1] Plays audio
  (Audio|PlaySoundatLocation (Variables|Default|Getsw_Close) (Transformation|GetActorForwardVector) "0, 0, 0" 1.0 1.0 0.0 0 0 0 0)
  ;[1 1 1] Open/ Close door in timeline
  (bind _track_door (Timeline|TL_OpenDoor Reverse)
    (:Update
      ;[1 1 1] Call custom collision event
      (CallFunction|PlayerDoorCollisionEvent)
      (Transformation|SetRelativeRotation (Variables|Default|GetSM_Door) (Math|Rotator|MakeRotator 0.0 0.0 (Math|Float|Lerp (Variables|Default|Getfl_ClosePos) (Variables|Default|Getfl_OpenPos) _track_door)) false false))
    (:Finished
      ;[1 1 1] Calls finished timeline event that handles auto locking and closing the door
      (CallFunction|FinishedTimeline))))

(event Custom|finishedTimeline
  ;[1 1 1] Event that is called when timeline has completed
  ;[1 1 1] Lock door
  (if (Variables|Default|Getbol_IsOpen)
    (if (Variables|Default|Gameplay|Getbol_CanLockBehind)
      (Variables|Default|Gameplay|Setbol_Lock true)
      (Development|PrintString "Door locked")
      (Audio|PlaySoundatLocation (Variables|Default|Getsw_Lock) (Transformation|GetActorForwardVector) "0, 0, 0" 1.0 1.0 0.0 0 0 0 0)))
  ;[1 1 1] Set door bool to inverse of whatever it is
  (Variables|Default|Setbol_IsOpen (not (Variables|Default|Getbol_IsOpen)))
  ;[1 1 1] Determines whether to re-show or hide tooltip by referencing event
  (if (Variables|Default|Getbol_InTriggerZone)
    (CallFunction|ReshowTooltips)
    (else
      (CallFunction|HideTooltips))))

(event Custom|PlayerDoorCollisionEvent
  ;[1 1 1] The custom event to check if player and the door are colliding
  ;[1 1 1] Checks bol for if player is in the near collision zone
  (if (Variables|Default|Getbol_PlayerDoorCollided)
    (Development|PrintString "Collision hit while moving")
    ;[1 1 1] Depending on if the door is open or close, the door will do the opposite
    (if (Variables|Default|Getbol_IsOpen)
      (CallFunction|OpenDoor)
      (else
        (CallFunction|CloseDoor)))))

(event Custom|reshowTooltips
  ;[1 1 1] Displays
  (if (Variables|Default|Gameplay|Getbol_Lock)
    (Development|PrintString "door looked")
    (Rendering|SetVisibility (Variables|Default|GetTR_UnlockPromptFront) true false)
    (else
      (Rendering|SetVisibility (Variables|Default|GetTR_OpenPromptFront) true false)
      (Rendering|SetVisibility (Variables|Default|GetTR_UnlockPromptFront) false false)))
  ;[1 1 1] Sets bool value whether the player is still in collision zone
  (Variables|Default|Setbol_InTriggerZone true))

(event Custom|HideTooltips
  ;[1 1 1] Displays
  (Rendering|SetVisibility (Variables|Default|GetTR_UnlockPromptFront) false false)
  (Rendering|SetVisibility (Variables|Default|GetTR_OpenPromptFront) false false))

(event Custom|swinging
  (bind _returnvalue (Game|GetPlayerCharacter 0))
  (bind _returnvalue_2 (Transformation|GetActorRightVector))
  (bind _mesh (Variables|/Script/Engine.Character|GetMesh _returnvalue))
  (bind _returnvalue_3 (Math|Vector|GetRightVector _mesh))
  (bind _returnvalue_4 (Math|Vector|DotProduct _returnvalue_3 _returnvalue_2))
  ;[1 1 1] Swing away from door
  (Development|PrintString (Utilities|String|ToString(Float) _returnvalue_4))
  (if (< 0.0 _returnvalue_4)
    (Variables|Default|Setfl_OpenPos (Variables|Default|Getfl_AwayFront))
    (else
      (Variables|Default|Setfl_OpenPos (Variables|Default|Getfl_AwayBack)))))

(event EventBeginPlay
  ;[1 0 0] BEGIN PLAY
  ;;[1 1 1] Calls event at start of playtime
  ;;[1 1 1] Calls at start
  (CallFunction|ChangeDoorType))

(fn ConstructionScript
  (bind _fl_openpos (Variables|Default|Getfl_OpenPos))
  ;[1 1 1] sets ajar amount
  (Transformation|SetRelativeRotation (Variables|Default|GetSM_Door) (Math|Rotator|MakeRotator 0.0 0.0 (Variables|Default|Gameplay|Getfl_AjarAmount)) false false)
  (CallFunction|BothDir)
  ;[1 1 1] sets open and close value
  (Variables|Default|Setfl_AwayBack (Math|Float|Absolute(Float) _fl_openpos))
  (Variables|Default|Setfl_AwayFront (* _fl_openpos 1.0)))

(fn ChangeDoorType
  (bind _output_get (Variables|Default|Gameplay|SetBPDA_DoorType (Variables|Default|Gameplay|GetBPDA_DoorType)))
  ;[1 1 1] Change visual/ audio of the door to respective type (can't be overriden)
  (Rendering|Material|SetMaterial (Variables|Default|GetSM_Door) 0 (Variables|/Game/DataAssets/BPDA_MainDataAsset.BPDA_MainDataAsset_C|GetMAT_Door _output_get))
  (Variables|Default|Setsw_Unlock (Variables|/Game/DataAssets/BPDA_MainDataAsset.BPDA_MainDataAsset_C|GetSW_Unlock _output_get))
  (Variables|Default|Setsw_Lock (Variables|/Game/DataAssets/BPDA_MainDataAsset.BPDA_MainDataAsset_C|GetSW_Lock _output_get))
  (Variables|Default|Setsw_Open (Variables|/Game/DataAssets/BPDA_MainDataAsset.BPDA_MainDataAsset_C|GetSW_Open _output_get))
  (Variables|Default|Setsw_Close (Variables|/Game/DataAssets/BPDA_MainDataAsset.BPDA_MainDataAsset_C|GetSW_Close _output_get))
  (Components|StaticMesh|SetStaticMesh (Variables|Default|GetSM_Door) (Variables|/Game/DataAssets/BPDA_MainDataAsset.BPDA_MainDataAsset_C|GetSM_Door _output_get))
  ;[1 1 1] if true, overrides the variable for different gameplay
  (if (Variables|Default|Gameplay|GetBol_OverrideGameplay)
    (Variables|Default|Gameplay|Setfl_TimeToOpen (Variables|/Game/DataAssets/BPDA_MainDataAsset.BPDA_MainDataAsset_C|GetFL_TimeToClose _output_get))
    (Variables|Default|Gameplay|Setfl_TimeToClose (Variables|/Game/DataAssets/BPDA_MainDataAsset.BPDA_MainDataAsset_C|GetFL_TimeToOpen _output_get))
    (Variables|Default|Gameplay|Setbol_Lock (Variables|/Game/DataAssets/BPDA_MainDataAsset.BPDA_MainDataAsset_C|GetBOL_Lock _output_get))
    (Variables|Default|Gameplay|Setbol_CanLockBehind (Variables|/Game/DataAssets/BPDA_MainDataAsset.BPDA_MainDataAsset_C|GetBOL_LockBehind _output_get))
    (Variables|Default|Gameplay|Setbol_SwingAway (Variables|/Game/DataAssets/BPDA_MainDataAsset.BPDA_MainDataAsset_C|GetBOL_SwingAway _output_get))))

(fn DoorSwinging
  (if (Variables|Default|Gameplay|Getbol_SwingAway)
    ;[1 1 1] If swing away is true, call an error message
    (CallFunction|BothDir)
    (Development|PrintString (Utilities|String|Append (Utilities|GetObjectName self) "Can't have bol Swing Away as ticked and tried to inverted") true true "(R=1.000000,G=0.197401,B=0.000000,A=1.000000)")
    (else
      ;[1 1 1] if swing away is false, change the direction the door swings
      (Development|PrintString (Utilities|String|ToString(Boolean) (Variables|Default|Getbol_SwitchBetween)))
      (if (Variables|Default|Getbol_SwitchBetween)
        (Variables|Default|Setfl_OpenPos (Variables|Default|Getfl_AwayBack))
        (Rendering|SetVisibility (Variables|Default|Getarrow_Back) true false)
        (Rendering|SetVisibility (Variables|Default|Getarrow_Front) false false)
        (Variables|Default|Setbol_SwitchBetween false)
        (else
          (Variables|Default|Setfl_OpenPos (Variables|Default|Getfl_AwayFront))
          (Rendering|SetVisibility (Variables|Default|Getarrow_Back) false false)
          (Rendering|SetVisibility (Variables|Default|Getarrow_Front) true false)
          (Variables|Default|Setbol_SwitchBetween true))))))

(fn BothDir
  ;[1 1 1] if swing away is true, shows both arrows
  (if (Variables|Default|Gameplay|Getbol_SwingAway)
    (Rendering|SetVisibility (Variables|Default|Getarrow_Back) true false)))

(fn Interact
  (params (Interactor :type Character%20Object%20Reference))
  (bind _tl_opendoor (Variables|Default|GetTL_OpenDoor))
  (if (not (Variables|Default|Getbol_AlternativeUnlock))
    ;[1 1 1] Gets bool and checks whether to open or close
    (if (not (Variables|Default|Getbol_IsOpen))
      ;[1 1 1] Handles door looking
      (if (not (Variables|Default|Gameplay|Getbol_Lock))
        ;[1 1 1] Reference timeline to open or close
        (Components|Timeline|SetPlayRate _tl_opendoor (/ 1.0 (Variables|Default|Gameplay|Getfl_TimeToOpen)))
        ;[1 1 1] Calls door event
        (CallFunction|OpenDoor)
        (return true))
      (else
        (Components|Timeline|SetPlayRate _tl_opendoor (/ 1.0 (Variables|Default|Gameplay|Getfl_TimeToClose)))
        (CallFunction|CloseDoor)
        (return true)))))

(fn Unlocking
  (params (Interactor :type Actor%20Object%20Reference))
  (if (not (Variables|Default|Getbol_AlternativeUnlock))
    ;[1 1 1] Gets bool and checks whether to open or close
    (if (not (Variables|Default|Getbol_IsOpen))
      ;[1 1 1] Handles door looking
      (if (Variables|Default|Gameplay|Getbol_Lock)
        (Variables|Default|Gameplay|Setbol_Lock false)
        (CallFunction|OpenDoor)
        (return true)
        (elif true
          (Variables|Default|Gameplay|Setbol_Lock true)
          (return true)))
      (elif (not (Variables|Default|Gameplay|Getbol_Lock))
        (Variables|Default|Gameplay|Setbol_Lock true)
        (CallFunction|CloseDoor)
        (return true)))))