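; BP_Lever is an interactable lever that toggles the lock on a linked reinforced door.
; Interact runs HandleLock, which tilts the lever part by the current boolean, casts ActDoorRef to BP_ReinforcedDoor_Child, calls UnlockDoor or LockDoor, then flips the boolean.
; A failed cast leaves the boolean unchanged, and BeginPlay prints a warning if the door reference is empty.
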(event Custom|HandleLock
  (bind _cube1 (Variables|Default|GetCube1))
  (bind _act_doorref (Variables|Default|Getact_DoorRef))
  ;[1 1 1] Handle lock event
  ;[1 1 1] checks the boolean
  (if (Variables|Default|Getbol_On)
    ;[1 1 1] change rotation of lever part
    (Transformation|SetRelativeRotation _cube1 "0.000000,0.000000,50.000000" false false)
    ;[1 0.6445 0] MM - Try and find a better implementation instead of using casts
    ;;[1 1 1] Casts to reinforce door to reference the specific event
    (bind _asbp_reinforced_door_child (Utilities|Casting|CastToBP_ReinforcedDoor_Child _act_doorref))
    (Default|UnlockDoor _asbp_reinforced_door_child)
    (else
      (Transformation|SetRelativeRotation _cube1 "0.000000,0.000000,-50.000000" false false)
      (bind _asbp_reinforced_door_child_2 (Utilities|Casting|CastToBP_ReinforcedDoor_Child _act_doorref))
      (Default|LockDoor _asbp_reinforced_door_child_2)))
  ;[1 1 1] inverts boolean
  (Variables|Default|Setbol_On (not (Variables|Default|Getbol_On))))

(event EventBeginPlay
  (if (== (Variables|Default|Getact_DoorRef) 0)
    (Development|PrintString (Utilities|String|Append (Utilities|GetObjectName self) "needs to have act DoorRef filled with a reinforced door"))))

(fn ConstructionScript)

(fn Interact
  (params (Interactor :type Character%20Object%20Reference))
  (CallFunction|HandleLock)
  (return false))